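; RTS player controller that handles camera movement input and toggles a spawner UI.
; On BeginPlay it creates the Spawner_UI widget, adds it to the viewport and hides it through zero render opacity.
; MoveForward, MoveRight and Zoom axis inputs pass straight to same-named functions defined outside these graphs.
; The P key flip-flops the widget's opacity and the mouse cursor together, without removing the widget.
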(event `self.ReceiveBeginPlay`
  (bind _returnvalue (`|CreateWidget` "/Game/Blueprints/Widget/Spawner_UI.Spawner_UI_C"))
  (bind _output_get (set `self.Widget` _returnvalue))
  (`UserWidget.AddToViewport` _output_get 0)
  (`Widget.SetRenderOpacity` (`self.Widget`) 0.0))

(event `InputAxis|MoveForward`
  (params (AxisValue :type "Float (single-precision)"))
  (`self.MoveForward` AxisValue))

(event `InputAxis|MoveRight`
  (params (AxisValue :type "Float (single-precision)"))
  (`self.MoveRight` AxisValue))

(event `InputAxis|Zoom`
  (params (AxisValue :type "Float (single-precision)"))
  (`self.Zoom` AxisValue))

(event `Key|P`
  (params (Key :type "Key Structure"))
  (:`Pressed`
    (`/Engine/EditorBlueprintResources/StandardMacros.FlipFlop`
      (:`A`
        (`Widget.SetRenderOpacity` (`self.Widget`) 1.0)
        (set `self.bShowMouseCursor` true))
      (:`B`
        (`Widget.SetRenderOpacity` (`self.Widget`) 0.0)
        (set `self.bShowMouseCursor` false)))))

(fn `UserConstructionScript`)