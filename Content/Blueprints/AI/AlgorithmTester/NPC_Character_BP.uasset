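; NPC character Blueprint in the AI AlgorithmTester folder that holds a current location and a target location.
; BeginPlay sets both to the spawn position, and Tick keeps StartLocation synced to the actor's position.
; The SetLoc event overwrites TargetLocation and GetLoc returns it; the Blueprint's graphs contain no movement logic.
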(event `self.ReceiveBeginPlay`
  (bind _output_get (set `self.StartLocation` (`self.K2_GetActorLocation`)))
  (set `self.TargetLocation` _output_get))

(event `self.ReceiveTick`
  (params (DeltaSeconds :type "Float (single-precision)"))
  (set `self.StartLocation` (`self.K2_GetActorLocation`)))

(event `/Game/Blueprints/AI/AlgorithmTester/BPI_Loc.SetLoc`
  (params (Loc :type "Vector Structure"))
  (set `self.TargetLocation` Loc))

(fn `GetLoc`
  (returns (Loc :type "Vector Structure"))
  (return (`self.TargetLocation`)))

(fn `UserConstructionScript`)