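; NPC group controller that relocates itself to random reachable points and passes movement targets to an array of NPCs; it spawns nothing itself.
; BeginPlay starts two looping timers, apparently for LocationPrint and MoveinGroup.
; LocationPrint picks a navigable point around the actor, stores it as TargetLocation and moves there.
; MoveinGroup sends each NPC implementing LocationInterface its own location plus TargetLocation, a sum of two world positions.
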(event `self.ReceiveBeginPlay`
  (`KismetSystemLibrary.K2_SetTimerDelegate` (`|CreateDelegate` :!event `LocationPrint`) 3.0 true)
  (`KismetSystemLibrary.K2_SetTimerDelegate` (`|CreateDelegate` :!event `MoveInGroup`) 3.0 true))

(event `LocationSpawnerInterface.LocationPrint`
  (bind _output_get (set `self.TargetLocation` (`NavigationSystemV1.K2_GetRandomReachablePointInRadius` (`SceneComponent.K2_GetComponentLocation` (`self.DefaultSceneRoot`)) 1000.0 null null)))
  (`self.K2_SetActorLocation` _output_get))

(event `self.ReceiveTick`
  (params (DeltaSeconds :type "Float (single-precision)")))

(event `LocationSpawnerInterface.MoveInGroup`
  (for _array_element (`self.NPC_Array`)
    (if (`KismetSystemLibrary.DoesImplementInterface` _array_element "/Script/RTS_Simulation.LocationInterface")
      (message `LocationInterface.Set_Location` _array_element (+ (`self.K2_GetActorLocation` _array_element) (`self.TargetLocation`))))))

(fn `UserConstructionScript`)