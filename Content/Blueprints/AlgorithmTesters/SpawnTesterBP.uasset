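; SpawnTesterBP is a test Blueprint for spawning a square grid of ABP_TileMap actors, though none of its logic currently runs.
; Disconnected chains derive grid count and tile scale from whole and single unit sizes, and clear the tile array.
; A nested loop spawns scaled tiles at stepped X/Y positions, stores them in the array and prints the total.
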(fn `UserConstructionScript`)