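; Spawner actor that builds a square grid of ABP_TileMap tiles when play begins.
; BeginPlay reads the whole-area and single-tile sizes from the RTS_Controller_BP widget and passes them to SpawnCalculate.
; Nested loops spawn rows of tiles at a fixed height, stepping by tile size and scaling each in X and Y to match.
; Spawned tiles are collected in an array, whose count is printed.
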(event `self.ReceiveBeginPlay`
  (bind _asrts_controller_bp (cast `/Game/Blueprints/Camera/RTS_Controller_BP` (`GameplayStatics.GetPlayerController` 0)))
  (bind _widget (`/Game/Blueprints/Camera/RTS_Controller_BP.Widget` _asrts_controller_bp))
  (`self.SpawnCalculate` (`/Game/Blueprints/Widget/Spawner_UI.WholeUnitValue` _widget) (`/Game/Blueprints/Widget/Spawner_UI.SingleUnitValue` _widget)))

(event `SpawnCalculate`
  (params (WholeUnit :type "Float (double-precision)") (SingleUnit :type "Float (double-precision)"))
  (bind _newvar_1 (`self.NewVar_1`))
  (set `self.Whole Unit` WholeUnit)
  (bind _output_get (set `self.Single Unit` SingleUnit))
  (set `self.NewVar_1` (/ _output_get 1000.0))
  (set `self.NewVar_2` (- (`KismetMathLibrary.Round` (/ (`self.Whole Unit`) (`self.Single Unit`))) 1))
  (for _index (range (+ (`self.NewVar_2`) 1))
    (set `self.i` _index)
    (for _index_2 (range (+ (`self.NewVar_2`) 1))
      (set `self.j` _index_2)
      (bind _returnvalue (`|SpawnActorFromClass` "/Game/Blueprints/ABP_TileMap.ABP_TileMap_C" (`KismetMathLibrary.MakeTransform` (`KismetMathLibrary.MakeVector` (`self.X_Loc`) (`self.Y_Loc`) 20.0) (struct) (`KismetMathLibrary.MakeVector` _newvar_1 _newvar_1 1.0)) "Undefined" "OverrideRootScale" null null))
      (`KismetArrayLibrary.Array_Add` (`self.NewVar_0`) _returnvalue)
      (set `self.Y_Loc` (+ (`self.Y_Loc`) (`self.Single Unit`))))
    (set `self.X_Loc` (+ (`self.X_Loc`) (`self.Single Unit`)))
    (set `self.Y_Loc` 0.0))
  (`KismetSystemLibrary.PrintString` (`KismetStringLibrary.Conv_IntToString` (`KismetArrayLibrary.Array_Length` (`self.NewVar_0`)))))

(fn `UserConstructionScript`)