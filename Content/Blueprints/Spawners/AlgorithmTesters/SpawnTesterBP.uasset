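; SpawnTesterBP is an algorithm tester for spawning a square grid of tiles, though none of its logic is connected to run.
; A sizing block derives row count and tile scale from WholeUnit and SingleUnit, both set to zero there.
; Nested loops step by SingleUnit, spawning scaled actors at a fixed height into TileArray, but the spawn node has no class assigned.
; The construction script is empty.
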(fn `UserConstructionScript`)